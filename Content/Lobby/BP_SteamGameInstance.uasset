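; Game instance that manages Steam multiplayer sessions and lobby UI through the Advanced Sessions plugin.
; Creating a session opens the vehicle example map as a listen server, while accepted invites feed into the join event, which shows loading and joins.
; Main menu, create-session and loading widgets are cached and reused.
; Finding sessions only spawns a new join-menu widget; the direct search and auto-join nodes are disconnected.
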(event `self.CreateSteamSession`
  ;[1 1 1] CREATE
  (`CreateSessionCallbackProxyAdvanced.CreateAdvancedSession` :`PlayerController` (`GameplayStatics.GetPlayerController` 0) :`PublicConnections` 4 :`PrivateConnections` 4
    (:`OnSuccess`
      (`self.ShowLoading` null)
      (`KismetSystemLibrary.PrintString` "Success" true true (struct :`G` 0.66 :`B` 1.0 :`A` 1.0) 5.0)
      (`GameplayStatics.OpenLevel` "VehicleAdvExampleMap" true "listen"))))

(event `self.FindSteamSession`
  ;[1 1 1] FIND
  (bind _returnvalue (`|CreateWidget` "/Game/Widgets/WB_JoinMenu.WB_JoinMenu_C" (`GameplayStatics.GetPlayerController` 0)))
  (`UserWidget.AddToViewport` _returnvalue 0))

(event `self.JoinSteamSession`
  (params (SessionToJoin :type "BlueprintSessionResult Structure"))
  ;[1 1 1] JOIN SESSION
  (`self.ShowLoading` null)
  (`JoinSessionCallbackProxy.JoinSession` (`GameplayStatics.GetPlayerController` 0) SessionToJoin))

(event `self.OnSessionInviteAccepted`
  (params (LocalPlayerNum :type Integer) (PersonInvited :type "BPUniqueNetId Structure") (SessionToJoin :type "BlueprintSessionResult Structure (by ref)"))
  ;[1 1 1] Comment
  (`self.JoinSteamSession` SessionToJoin))

(event `self.ShowCreateSession`
  (bind _returnvalue (`GameplayStatics.GetPlayerController` 0))
  ;[1 1 1] SHOW CREATE GAME
  (`self.CreateSessionWB`
    (:`then`
      _)
    (:`else`
      (bind _returnvalue_2 (`|CreateWidget` "/Game/Widgets/WB_CreateSession.WB_CreateSession_C" _returnvalue))
      (set `self.CreateSessionWB` _returnvalue_2)))
  (`UserWidget.AddToViewport` (`self.CreateSessionWB`) 0)
  (`/Engine/EditorBlueprintResources/StandardMacros.IsValid` _returnvalue
    (:`Is Valid`
      (set `PlayerController.bShowMouseCursor` true _returnvalue))))

(event `self.ShowMainMenu`
  (bind _returnvalue (`GameplayStatics.GetPlayerController` 0))
  ;[1 1 1] SHOW MAIN MENU
  (`self.MainMenuWB`
    (:`then`
      _)
    (:`else`
      (bind _returnvalue_2 (`|CreateWidget` "/Game/Widgets/WB_MainMenu.WB_MainMenu_C" (`GameplayStatics.GetPlayerController` 0)))
      (set `self.MainMenuWB` _returnvalue_2)
      (bind _mainmenuwb (`self.MainMenuWB`)
        (:`then`
          _)
        (:`else`))))
  (`UserWidget.AddToViewport` _mainmenuwb 0)
  (`/Game/Widgets/WB_MainMenu.SetPlayerName` _mainmenuwb)
  (`/Engine/EditorBlueprintResources/StandardMacros.IsValid` _returnvalue
    (:`Is Valid`
      (set `PlayerController.bShowMouseCursor` true _returnvalue)
      (`WidgetBlueprintLibrary.SetInputMode_GameAndUIEx` _returnvalue _mainmenuwb "DoNotLock" false))))

(event `self.ShowLoading`
  (params (actor :type "Actor Object Reference"))
  ;[1 1 1] SHOW LOADING
  (`self.LoadingWB`
    (:`then`
      _)
    (:`else`
      (bind _returnvalue (`|CreateWidget` "/Game/Widgets/WB_Loading.WB_Loading_C" (`GameplayStatics.GetPlayerController` 0)))
      (set `self.LoadingWB` _returnvalue)))
  (`UserWidget.AddToViewport` (`self.LoadingWB`) 0))

(fn `Reference`
  (returns (GameInstance :type "/Game/Lobby/BP_SteamGameInstance Object Reference"))
  (return null))