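; Drivable LuAZ-969 Chaos vehicle pawn, controlled by player input or simple AI.
; Server-to-multicast events push body color, brake and headlight values into a dynamic material.
; On tick, AI follows a lane spline under a speed limit with front traces for obstacles, and engine audio tracks forward speed.
; Hard impacts detach wheels and swap in damaged wheel classes; input also cycles cameras and requests game-mode respawn.
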(event `UpdateMaterial_Server`
  (params (brake :type "Float (double-precision)") (body_c :type "LinearColor Structure") (Light :type "Float (double-precision)"))
  (`self.UpdateMaterial_Multicast` brake body_c Light))

(event `UpdateMaterial_Multicast`
  (params (Brake :type "Float (double-precision)") (body_c :type "LinearColor Structure") (Light :type "Float (double-precision)"))
  (bind _matbody (`self.MatBody`)
    (:`then`
      (`MaterialInstanceDynamic.SetScalarParameterValue` _matbody "BrakeLightPower" Brake)
      (`MaterialInstanceDynamic.SetVectorParameterValue` _matbody "BodyColor" body_c)
      (`MaterialInstanceDynamic.SetScalarParameterValue` _matbody "FrontLightPower" Light))
    (:`else`)))

(event `UpdateMaterial`
  (`/Engine/EditorBlueprintResources/ActorMacros.Switch Has Authority`
    (:`Authority`
      (`self.UpdateMaterial_Multicast` 0.0))
    (:`Remote`
      (`self.UpdateMaterial_Server` 0.0))))

(event `self.ReceiveBeginPlay`
  ;[1 1 1] START
  (bind _returnvalue (`PrimitiveComponent.CreateDynamicMaterialInstance` (`self.Mesh`) 0 "/Game/Vehicles/szd/Mat/mat_szd_base_Inst.mat_szd_base_Inst" "None"))
  (set `self.MatBody` _returnvalue)
  (`self.respawn_init` (`AdvancedIdentityLibrary.GetPlayerNickname` (`AdvancedSessionsLibrary.GetUniqueNetID` (`GameplayStatics.GetPlayerController` 0))))
  (`self.ShowName` false)
  (for _array_element (`self.K2_GetComponentsByClass` "/Script/Engine.CameraComponent")
    (`KismetArrayLibrary.Array_Add` (`self.cams`) _array_element)
    (set `self.ActiveCamera` 0)
    (if (`self.isAI`)
      (`|ExecutionSequence`
        (:`then_0`
          (`KismetSystemLibrary.Delay` (`KismetMathLibrary.RandomFloatInRange` 0.0 30.0))
          (set `self.AI_throttle` 1.0))))))

(event `self.Mesh.OnComponentHit`
  (params (HitComponent :type "PrimitiveComponent Object Reference") (OtherActor :type "Actor Object Reference") (OtherComp :type "PrimitiveComponent Object Reference") (NormalImpulse :type "Vector Structure") (Hit :type "HitResult Structure (by ref)"))
  (bind (_bblockinghit _binitialoverlap _time _distance _location _impactpoint _normal _impactnormal _physmat _hitactor _hitcomponent _hitbonename _bonename) (`GameplayStatics.BreakHitResult` Hit))
  ;[1 1 1] HIT
  (if (> (`KismetMathLibrary.VSize` NormalImpulse) 550000.0)
    (`GameplayStatics.SpawnEmitterAtLocation` "/Game/StarterContent/Particles/P_HIT.P_HIT" _location (struct) (1.0 1.0 1.0) true "AutoRelease")
    (bind _aschaos_wheeled_vehicle_movement_component (cast `ChaosWheeledVehicleMovementComponent` (`self.VehicleMovementComponent`)))
    (`|ExecutionSequence`
      (:`then_0`
        (if (== _bonename "Phys_Wheel_FR")
          (`self.DetachWheel` (`self.WheelFR`))
          (`ChaosWheeledVehicleMovementComponent.SetWheelClass` _aschaos_wheeled_vehicle_movement_component 1 "/Game/Vehicles/szd/Wheel/szd_WheelsFront_Damaged.szd_WheelsFront_Damaged_C")))
      (:`then_1`
        (if (== _bonename "Phys_Wheel_FL")
          (`self.DetachWheel` (`self.WheelFL`))
          (`ChaosWheeledVehicleMovementComponent.SetWheelClass` _aschaos_wheeled_vehicle_movement_component 0 "/Game/Vehicles/szd/Wheel/szd_WheelsFront_Damaged.szd_WheelsFront_Damaged_C")))
      (:`then_2`
        (if (== _bonename "Phys_Wheel_BR")
          (`self.DetachWheel` (`self.WheelBR`))
          (`ChaosWheeledVehicleMovementComponent.SetWheelClass` _aschaos_wheeled_vehicle_movement_component 3 "/Game/Vehicles/szd/Wheel/szd_WheelsRearDamaged.szd_WheelsRearDamaged_C")))
      (:`then_3`
        (if (== _bonename "Phys_Wheel_BL")
          (`self.DetachWheel` (`self.WheelBL`))
          (`ChaosWheeledVehicleMovementComponent.SetWheelClass` _aschaos_wheeled_vehicle_movement_component 2 "/Game/Vehicles/szd/Wheel/szd_WheelsRearDamaged.szd_WheelsRearDamaged_C"))))))

(event `respawn_init`
  (params (name :type String))
  (set `self.DisplayName` name)
  (`self.random_color`))

(event `InputAxis|MoveForward`
  (params (AxisValue :type "Float (single-precision)"))
  (bind _vehiclemovementcomponent (`self.VehicleMovementComponent`))
  (bind _vehiclemovementcomponent_2 (`self.VehicleMovementComponent`))
  ;[1 1 1] Movement control
  (if (`self.isAI`)
    _
    (elif (>= AxisValue 0.0)
      (`ChaosVehicleMovementComponent.SetThrottleInput` _vehiclemovementcomponent AxisValue)
      (`ChaosVehicleMovementComponent.SetBrakeInput` _vehiclemovementcomponent 0.0)
      (`/Engine/EditorBlueprintResources/StandardMacros.DoOnce` false :!label _label
        (:`Completed`
          (`self.BrakeLights` false)))
      (else
        (`ChaosVehicleMovementComponent.SetBrakeInput` _vehiclemovementcomponent_2 (* AxisValue -1.0))
        (`ChaosVehicleMovementComponent.SetThrottleInput` _vehiclemovementcomponent_2 0.0)
        (`self.BrakeLights` true)
        (goto _label :!via `Reset`)))))

(event `InputAxis|MoveRight`
  (params (AxisValue :type "Float (single-precision)"))
  ;[1 1 1] Movement control
  (if (not (`self.isAI`))
    (`ChaosVehicleMovementComponent.SetSteeringInput` (`self.VehicleMovementComponent`) AxisValue)))

(event `InputAction|SwitchLight`
  (params (Key :type "Key Structure"))
  ;[1 1 1] LIGHT
  (:`Pressed`
    (bind _output_get (set `self.FrontLight` 15.0))
    (`self.UpdateMaterial_Server` (`self.BrakeLight`) (`self.ColorBody`) _output_get)))

(event `InputAction|Handbrake`
  (params (Key :type "Key Structure"))
  (bind _vehiclemovementcomponent (`self.VehicleMovementComponent`))
  ;[1 1 1] Movement control
  (:`Pressed`
    (`ChaosVehicleMovementComponent.SetHandbrakeInput` _vehiclemovementcomponent true)
    (`self.BrakeLights` true))
  (:`Released`
    (`ChaosVehicleMovementComponent.SetHandbrakeInput` _vehiclemovementcomponent false)
    (`self.BrakeLights` false)))

(event `InputAction|color_test`
  (params (Key :type "Key Structure"))
  ;[1 1 1] RANDOM COLORS
  (:`Pressed`
    (`self.random_color`)))

(event `random_color`
  ;[1 1 1] RANDOM COLORS
  (bind _output_get (set `self.ColorBody` (make `LinearColor` (`KismetMathLibrary.RandomFloatInRange` 0.44 0.96) (`KismetMathLibrary.RandomFloatInRange` 0.24 1.0) (`KismetMathLibrary.RandomFloatInRange` 0.1 0.9) 1.0)))
  (`self.UpdateMaterial_Server` (`self.BrakeLight`) _output_get (`self.FrontLight`)))

(event `InputAxis|LookRight`
  (params (AxisValue :type "Float (single-precision)"))
  (bind _springback (`self.SpringBack`))
  (bind (_returnvalue_roll _returnvalue_pitch _returnvalue_yaw) (`KismetMathLibrary.BreakRotator` (`SceneComponent.K2_GetComponentRotation` _springback)))
  ;[1 1 1] Camera Control
  (if (> (`KismetMathLibrary.Abs` _returnvalue_pitch) 50.0) :!label _label_2
    (`SceneComponent.K2_SetWorldRotation` _springback (`KismetMathLibrary.RInterpTo` (`KismetMathLibrary.MakeRotator` _returnvalue_roll _returnvalue_pitch _returnvalue_yaw) (`KismetMathLibrary.MakeRotator` _returnvalue_roll 0.0 _returnvalue_yaw) (`GameplayStatics.GetWorldDeltaSeconds`) 1.0) false false)
    (else
      (`SceneComponent.K2_AddRelativeRotation` _springback (`KismetMathLibrary.MakeRotator` 0.0 (stale `InputAxis|LookUp` AxisValue) AxisValue) false false))))

(event `InputAxis|LookUp`
  (params (AxisValue :type "Float (single-precision)"))
  ;[1 1 1] Camera Control
  (goto _label_2))

(event `InputAction|SwitchCamera`
  (params (Key :type "Key Structure"))
  (bind _cams (`self.cams`))
  (bind _cams_2 (`self.cams`))
  (bind _returnvalue (+ (`self.ActiveCamera`) 1))
  ;[1 1 1] Camera Control
  (:`Pressed`
    (for _array_element _cams_2
      (`ActorComponent.Deactivate` _array_element))
    (set `self.ActiveCamera` _returnvalue)
    (if (> _returnvalue (`KismetArrayLibrary.Array_Length` _cams_2))
      (bind _output_get (set `self.ActiveCamera` 0))
      (`ActorComponent.Activate` (`|GetArrayItem` _cams _output_get) false)
      (else
        (`ActorComponent.Activate` (`|GetArrayItem` _cams (`self.ActiveCamera`)) false)))))

(event `InputAction|ResetCar`
  (params (Key :type "Key Structure"))
  ;[1 1 1] RESPAWN
  (:`Pressed`
    (`/Engine/EditorBlueprintResources/ActorMacros.Switch Has Authority`
      (:`Authority`
        _)
      (:`Remote`
        _))
    (`self.reset` (`GameplayStatics.GetPlayerController` 0))))

(event `reset`
  (params (controll :type "PlayerController Object Reference"))
  (bind (_returnvalue_roll _returnvalue_pitch _returnvalue_yaw) (`KismetMathLibrary.BreakRotator` (`self.K2_GetActorRotation`)))
  (bind _returnvalue (`GameplayStatics.GetGameMode`))
  ;[1 1 1] SERVER RESET
  (`/Engine/EditorBlueprintResources/ActorMacros.Switch Has Authority`
    (:`Authority`
      (`/Engine/EditorBlueprintResources/StandardMacros.IsValid` _returnvalue
        (:`Is Valid`
          (bind _asvehicle_adv_game_mode (cast `/Game/VehicleTemplate/Blueprints/VehicleAdvGameMode` _returnvalue))
          (`/Game/VehicleTemplate/Blueprints/VehicleAdvGameMode.respawn` _asvehicle_adv_game_mode controll (`KismetMathLibrary.MakeTransform` (+ (`self.K2_GetActorLocation`) (0.0 0.0 250.0)) (`KismetMathLibrary.MakeRotator` 0.0 0.0 _returnvalue_yaw)))
          (`KismetSystemLibrary.PrintString` "reset !"))))))

(event `self.ReceiveTick`
  (params (DeltaSeconds :type "Float (single-precision)"))
  (bind _engineaudio (`self.EngineAudio`))
  (bind _ai_throttle (`self.AI_throttle`))
  (`|ExecutionSequence`
    (:`then_0`
      ;[1 1 1] AI TICK
      (if (`self.isAI`)
        (`self.FrontTracer`)
        (if (`self.FrontTraceHit`)
          (if (< (`self.GetSpeedKMH`) 0.0)
            (`self.SetAI` 0.0 5.0 5.0)
            (else
              (`self.SetAI` (* _ai_throttle 0.1) 0.0 -5.0)))
          (else
            (`self.Speed Limiter` (`self.Speed Limit KMH`)
              (:`then`
                (bind _steering (`self.AIGetLane` (`self.LaneSpline`)))
                (`self.SetAI` _ai_throttle 0.0 _steering))
              (:`false`
                (`self.SetAI` 0.0 1.0)))))))
    (:`then_1`
      ;[1 1 1] Audio
      (`AudioParameterControllerInterface.ResetParameters` _engineaudio)
      (`AudioParameterControllerInterface.SetFloatParameter` _engineaudio "RPM" (`KismetMathLibrary.Abs` (`ChaosVehicleMovementComponent.GetForwardSpeed` (`self.VehicleMovementComponent`)))))))

(fn `AIGetLane`
  (params (Path :type "/Game/AI/LanePath Object Reference"))
  (returns (steering :type "Float (double-precision)"))
  (bind _returnvalue (`self.K2_GetActorLocation`))
  (bind _spline (`/Game/AI/LanePath.Spline` Path))
  (bind (_returnvalue_roll _returnvalue_pitch _returnvalue_yaw) (`KismetMathLibrary.BreakRotator` (`KismetMathLibrary.NormalizedDeltaRotator` (`KismetMathLibrary.FindLookAtRotation` _returnvalue (`SplineComponent.FindLocationClosestToWorldLocation` _spline (+ (* (`KismetMathLibrary.Normal` (`SplineComponent.FindTangentClosestToWorldLocation` _spline _returnvalue "World")) 500.0) _returnvalue) "World")) (`self.K2_GetActorRotation`))))
  (return (`KismetMathLibrary.MapRangeClamped` _returnvalue_yaw -90.0 90.0 -5.0 5.0)))

(fn `BrakeLights`
  (params (BrakeLights :type Boolean))
  (bind _frontlight (`self.FrontLight`))
  (bind _colorbody (`self.ColorBody`))
  (if BrakeLights
    (bind _output_get (set `self.BrakeLight` 6.0))
    (`self.UpdateMaterial_Server` _output_get _colorbody _frontlight)
    (else
      (bind _output_get_2 (set `self.BrakeLight` 0.0))
      (`self.UpdateMaterial_Server` _output_get_2 _colorbody _frontlight))))

(fn `DetachWheel`
  (params (wheel :type "StaticMeshComponent Object Reference"))
  (`SceneComponent.K2_DetachFromComponent` wheel "KeepWorld" "KeepWorld" "KeepWorld" true)
  (`PrimitiveComponent.SetCollisionEnabled` wheel "QueryAndPhysics")
  (`PrimitiveComponent.SetSimulatePhysics` wheel true))

(fn `FrontTracer`
  (locals (NewLocalVar_0 :type Boolean :default false))
  (bind _ai_fronttracer (`self.AI_FrontTracer`))
  (bind _ai_fronttracer1 (`self.AI_FrontTracer1`))
  (bind _returnvalue (`SceneComponent.K2_GetComponentLocation` _ai_fronttracer))
  (bind _returnvalue_2 (`SceneComponent.K2_GetComponentLocation` _ai_fronttracer1))
  (bind (_outhits _returnvalue_3) (`KismetSystemLibrary.LineTraceMulti` _returnvalue (+ _returnvalue (* (`SceneComponent.GetForwardVector` _ai_fronttracer) 600.0)) "TraceTypeQuery1"))
  (bind (_outhits_2 _returnvalue_4) (`KismetSystemLibrary.LineTraceMulti` _returnvalue_2 (+ _returnvalue_2 (* (`SceneComponent.GetForwardVector` _ai_fronttracer1) 400.0)) "TraceTypeQuery1"))
  (bind _output_get (set `self.FrontTraceHit` (or _returnvalue_3 _returnvalue_4)))
  (if _output_get
    (set `self.AI_Steering` 5.0)))

(fn `GetSpeedKMH`
  (returns (speed :type "Float (double-precision)"))
  (return (* (`ChaosVehicleMovementComponent.GetForwardSpeed` (`self.VehicleMovementComponent`)) 0.036)))

(fn `OnRep_DisplayName`
  (`TextRenderComponent.K2_SetText` (`self.TextRender`) (`KismetTextLibrary.Conv_StringToText` (`self.DisplayName`))))

(fn `SetAI`
  (params (throttle :type "Float (double-precision)") (brake :type "Float (double-precision)") (steer :type "Float (double-precision)"))
  (bind _vehiclemovementcomponent (`self.VehicleMovementComponent`))
  (`ChaosVehicleMovementComponent.SetThrottleInput` _vehiclemovementcomponent throttle)
  (`ChaosVehicleMovementComponent.SetBrakeInput` _vehiclemovementcomponent brake)
  (`ChaosVehicleMovementComponent.SetSteeringInput` _vehiclemovementcomponent steer)
  (`self.BrakeLights` (> brake 0.0)))

(fn `SetLights`
  (params (lights :type "Float (double-precision)"))
  (bind _output_get (set `self.FrontLight` lights))
  (`self.UpdateMaterial_Server` (`self.BrakeLight`) (`self.ColorBody`) _output_get))

(fn `SetPaint`
  (params (color :type "LinearColor Structure"))
  (bind _output_get (set `self.ColorBody` color))
  (`self.UpdateMaterial_Server` (`self.BrakeLight`) _output_get (`self.FrontLight`)))

(fn `ShowName`
  (params (Show :type Boolean))
  (`SceneComponent.SetVisibility` (`self.TextRender`) Show false))

(fn `UserConstructionScript`)