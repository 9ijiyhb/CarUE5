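; BP_Zeppelin is a zeppelin actor that travels along the spline of its PathToFollow reference.
; On BeginPlay a timeline, rate-scaled by Time, maps its track to spline distance and sets actor location and rotation each update, reading location in world space but rotation in local space.
; An unconnected VInterpTo snippet and an uncalled FollowPath function, which computes a clamped yaw steering value from a look-ahead point, are unused.
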(event `self.ReceiveBeginPlay`
  (bind _spline (`/Game/AI/LanePath.Spline` (`self.PathToFollow`)))
  (`TimelineComponent.SetPlayRate` (`self.FollowSplinePath`) (/ 1.0 (`self.Time`)))
  (bind (_direction _splinetrack) (`Timeline|FollowSplinePath`)
    (:`Update`
      (bind _returnvalue (`KismetMathLibrary.Lerp` 0.0 (`SplineComponent.GetSplineLength` _spline) _splinetrack))
      (`self.K2_SetActorTransform` (`KismetMathLibrary.MakeTransform` (`SplineComponent.GetLocationAtDistanceAlongSpline` _spline _returnvalue "World") (`SplineComponent.GetRotationAtDistanceAlongSpline` _spline _returnvalue "Local"))))))

(event `self.ReceiveTick`
  (params (DeltaSeconds :type "Float (single-precision)")))

(fn `FollowPath`
  (params (Path :type "/Game/AI/LanePath Object Reference"))
  (returns (steering :type "Float (double-precision)"))
  (bind _returnvalue (`self.K2_GetActorLocation`))
  (bind _spline (`/Game/AI/LanePath.Spline` Path))
  (bind (_returnvalue_roll _returnvalue_pitch _returnvalue_yaw) (`KismetMathLibrary.BreakRotator` (`KismetMathLibrary.NormalizedDeltaRotator` (`KismetMathLibrary.FindLookAtRotation` _returnvalue (`SplineComponent.FindLocationClosestToWorldLocation` _spline (+ (* (`KismetMathLibrary.Normal` (`SplineComponent.FindTangentClosestToWorldLocation` _spline _returnvalue "World")) 1000.0) _returnvalue) "World")) (`self.K2_GetActorRotation`))))
  (return (`KismetMathLibrary.MapRangeClamped` _returnvalue_yaw -90.0 90.0 -5.0 5.0)))

(fn `UserConstructionScript`)