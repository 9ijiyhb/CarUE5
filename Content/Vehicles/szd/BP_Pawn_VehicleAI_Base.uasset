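; Base AI Chaos vehicle pawn that drives itself along a Lane spline.
; Each tick, three front traces trigger avoidance or braking; otherwise it steers toward a look-ahead spline point, with tangent length setting the speed limit.
; A delayed stuck check destroys barely moved cars on the server.
; Hard hits detach wheels and degrade their physics, while server/multicast events update paint and lights, and speed drives engine audio.
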(event `UpdateMaterial_Server`
  (params (brake :type "Float (double-precision)") (body_c :type "LinearColor Structure") (Light :type "Float (double-precision)"))
  ;[1 0.2444 0] RANDOM COLORS
  (`self.UpdateMaterial_Multicast` brake body_c Light))

(event `UpdateMaterial_Multicast`
  (params (Brake :type "Float (double-precision)") (body_c :type "LinearColor Structure") (Light :type "Float (double-precision)"))
  ;[1 0.2444 0] RANDOM COLORS
  (bind _matbody (`self.MatBody`)
    (:`then`
      (`MaterialInstanceDynamic.SetScalarParameterValue` _matbody "BrakeLightPower" Brake)
      (`MaterialInstanceDynamic.SetVectorParameterValue` _matbody "BodyColor" body_c)
      (`MaterialInstanceDynamic.SetScalarParameterValue` _matbody "FrontLightPower" Light))
    (:`else`)))

(event `UpdateMaterial`
  ;[1 0.2444 0] RANDOM COLORS
  (`/Engine/EditorBlueprintResources/ActorMacros.Switch Has Authority`
    (:`Authority`
      (`self.UpdateMaterial_Multicast` 0.0))
    (:`Remote`
      (`self.UpdateMaterial_Server` 0.0))))

(event `InputAction|color_test`
  (params (Key :type "Key Structure"))
  ;[1 0.2444 0] RANDOM COLORS
  (:`Pressed`
    (`self.random_color`)))

(event `random_color`
  ;[1 0.2444 0] RANDOM COLORS
  (bind _output_get (set `self.ColorBody` (make `LinearColor` (`KismetMathLibrary.RandomFloatInRange` 0.44 0.96) (`KismetMathLibrary.RandomFloatInRange` 0.24 1.0) (`KismetMathLibrary.RandomFloatInRange` 0.1 0.9) 1.0)))
  (`self.UpdateMaterial_Server` (`self.BrakeLight`) _output_get (`self.FrontLight`)))

(event `InputAction|SwitchLight`
  (params (Key :type "Key Structure"))
  ;[1 1 1] LIGHT
)

(event `self.Mesh.OnComponentHit`
  (params (HitComponent :type "PrimitiveComponent Object Reference") (OtherActor :type "Actor Object Reference") (OtherComp :type "PrimitiveComponent Object Reference") (NormalImpulse :type "Vector Structure") (Hit :type "HitResult Structure (by ref)"))
  (bind (_bblockinghit _binitialoverlap _time _distance _location _impactpoint _normal _impactnormal _physmat _hitactor _hitcomponent _hitbonename _bonename) (`GameplayStatics.BreakHitResult` Hit))
  ;[1 1 1] HIT
  (if (> (`KismetMathLibrary.VSize` NormalImpulse) (`self.Wheel_detach_force`))
    (`GameplayStatics.SpawnEmitterAtLocation` "/Game/StarterContent/Particles/P_HIT.P_HIT" _location (struct) (1.0 1.0 1.0) true "AutoRelease")
    (bind _aschaos_wheeled_vehicle_movement_component (cast `ChaosWheeledVehicleMovementComponent` (`self.VehicleMovementComponent`)))
    (`|ExecutionSequence`
      (:`then_0`
        (if (== _bonename "Phys_Wheel_FR")
          (`self.DetachWheel` (`self.WheelFR`))
          (`ChaosWheeledVehicleMovementComponent.SetWheelRadius` _aschaos_wheeled_vehicle_movement_component 1 10.0)
          (`ChaosWheeledVehicleMovementComponent.SetWheelFrictionMultiplier` _aschaos_wheeled_vehicle_movement_component 1 0.5)))
      (:`then_1`
        (if (== _bonename "Phys_Wheel_FL")
          (`self.DetachWheel` (`self.WheelFL`))
          (`ChaosWheeledVehicleMovementComponent.SetWheelRadius` _aschaos_wheeled_vehicle_movement_component 0 10.0)
          (`ChaosWheeledVehicleMovementComponent.SetWheelFrictionMultiplier` _aschaos_wheeled_vehicle_movement_component 0 0.5)))
      (:`then_2`
        (if (== _bonename "Phys_Wheel_BR")
          (`self.DetachWheel` (`self.WheelBR`))
          (`ChaosWheeledVehicleMovementComponent.SetWheelRadius` _aschaos_wheeled_vehicle_movement_component 3 10.0)
          (`ChaosWheeledVehicleMovementComponent.SetWheelFrictionMultiplier` _aschaos_wheeled_vehicle_movement_component 3 0.5)))
      (:`then_3`
        (if (== _bonename "Phys_Wheel_BL")
          (`self.DetachWheel` (`self.WheelBL`))
          (`ChaosWheeledVehicleMovementComponent.SetWheelRadius` _aschaos_wheeled_vehicle_movement_component 2 10.0)
          (`ChaosWheeledVehicleMovementComponent.SetWheelFrictionMultiplier` _aschaos_wheeled_vehicle_movement_component 2 0.5))))))

(event `self.ReceiveBeginPlay`
  ;[0.4914 1 0.5337] START
  (bind _returnvalue (`PrimitiveComponent.CreateDynamicMaterialInstance` (`self.Mesh`) 0 "/Game/Vehicles/szd/Mat/mat_szd_base_Inst.mat_szd_base_Inst" "None"))
  (set `self.MatBody` _returnvalue)
  (`self.respawn_init` (`KismetSystemLibrary.GetDisplayName` (`self.GetController`)))
  (set `self.AI_throttle` 1.0))

(event `InputAction|ResetCar`
  (params (Key :type "Key Structure"))
  ;[1 1 1] RESPAWN
  (:`Pressed`
    (`/Engine/EditorBlueprintResources/ActorMacros.Switch Has Authority`
      (:`Authority`
        _)
      (:`Remote`
        _))
    (`self.reset`)))

(event `reset`
  (bind _returnvalue (`GameplayStatics.GetGameMode`))
  ;[1 1 1] SERVER RESET
  (`/Engine/EditorBlueprintResources/ActorMacros.Switch Has Authority`
    (:`Authority`
      (`/Engine/EditorBlueprintResources/StandardMacros.IsValid` _returnvalue
        (:`Is Valid`
          (bind _asvehicle_adv_game_mode (cast `/Game/VehicleTemplate/Blueprints/VehicleAdvGameMode` _returnvalue))
          (`self.DetachFromControllerPendingDestroy` (`Controller.K2_GetPawn` (`self.GetController`)))
          (`self.K2_DestroyActor`)
          (`KismetSystemLibrary.PrintString` "reset !"))))))

(event `self.ReceiveTick`
  (params (DeltaSeconds :type "Float (single-precision)"))
  (bind _engineaudio (`self.EngineAudio`))
  (bind _ai_steering (`self.AI_Steering`))
  (`|ExecutionSequence`
    (:`then_0`
      ;[1 0.5167 0.1567] AI TICK
      (`self.FrontTracer`)
      (if (`self.FrontTraceHit`)
        (if (< (`self.GetSpeedKMH`) 5.0)
          (`self.SetAI` 0.0 5.0 _ai_steering)
          (else
            (`self.SetAI` 0.25 0.0 (* _ai_steering -1.0))))
        (`KismetSystemLibrary.Delay` 5.0 :!label _label)
        (`self.AutoDestroy`)
        (else
          (`self.Speed Limiter` (`self.AI Speed Limit`)
            (:`then`
              (bind (_steering _throttle) (`self.AIGetLane` (`self.Lane`)))
              (`self.SetAI` (`self.AI_throttle`) 0.0 (* _steering 5.0))
              (set `self.AI Speed Limit` (`KismetMathLibrary.MapRangeClamped` _throttle 0.0 500.0 (`self.Speed Limit MIN KMH`) (`self.Speed Limit MAX KMH`)))
              (goto _label))
            (:`false`
              (`self.SetAI` 0.0 1.0))))))
    (:`then_1`
      ;[0.09311 0 1] Audio
      (`AudioParameterControllerInterface.ResetParameters` _engineaudio)
      (`AudioParameterControllerInterface.SetFloatParameter` _engineaudio "RPM" (`KismetMathLibrary.Abs` (`ChaosVehicleMovementComponent.GetForwardSpeed` (`self.VehicleMovementComponent`)))))))

(event `respawn_init`
  (params (name :type String))
  ;[1 1 1] SERVER RESET
  (set `self.DisplayName` name))

(fn `AIGetLane`
  (params (Path :type "/Game/AI/LanePath Object Reference"))
  (returns (steering :type "Float (double-precision)") (throttle :type "Float (double-precision)"))
  (bind _spline (`/Game/AI/LanePath.Spline` Path))
  (bind _x (.x (`self.K2_GetActorLocation`)))
  (bind _y (.y (`self.K2_GetActorLocation`)))
  (bind _returnvalue (`KismetMathLibrary.MakeVector` _x _y (.z (`SplineComponent.FindLocationClosestToWorldLocation` _spline (`KismetMathLibrary.MakeVector` _x _y (.z (`SceneComponent.K2_GetComponentLocation` _spline))) "World"))))
  (bind _returnvalue_2 (+ (* (`KismetMathLibrary.Normal` (`SplineComponent.FindTangentClosestToWorldLocation` _spline _returnvalue "World")) 640.0) _returnvalue))
  (bind (_returnvalue_roll _returnvalue_pitch _returnvalue_yaw) (`KismetMathLibrary.BreakRotator` (`KismetMathLibrary.NormalizedDeltaRotator` (`KismetMathLibrary.FindLookAtRotation` _returnvalue (`SplineComponent.FindLocationClosestToWorldLocation` _spline _returnvalue_2 "World")) (`self.K2_GetActorRotation`))))
  (`/Engine/EditorBlueprintResources/StandardMacros.IsValid` Path
    (:`Is Valid`
      (return (`KismetMathLibrary.MapRangeClamped` _returnvalue_yaw -90.0 90.0 -1.0 1.0) (* (`KismetMathLibrary.VSize` (`SplineComponent.FindTangentClosestToWorldLocation` _spline _returnvalue_2 "World")) 0.01)))))

(fn `AutoDestroy`
  (bind _returnvalue (`self.K2_GetActorLocation`))
  (if (< (`KismetMathLibrary.Vector_Distance` (`self.PreviousLocation`) _returnvalue) 100.0)
    (`KismetSystemLibrary.PrintString` "DESTROY")
    (`self.reset`)
    (else
      (set `self.PreviousLocation` _returnvalue))))

(fn `BrakeLights`
  (params (BrakeLights :type Boolean))
  (bind _frontlight (`self.FrontLight`))
  (bind _colorbody (`self.ColorBody`))
  (if BrakeLights
    (bind _output_get (set `self.BrakeLight` 6.0))
    (`self.UpdateMaterial_Server` _output_get _colorbody _frontlight)
    (else
      (bind _output_get_2 (set `self.BrakeLight` 0.0))
      (`self.UpdateMaterial_Server` _output_get_2 _colorbody _frontlight))))

(fn `DetachWheel`
  (params (wheel :type "StaticMeshComponent Object Reference"))
  (`SceneComponent.K2_DetachFromComponent` wheel "KeepWorld" "KeepWorld" "KeepWorld" true)
  (`PrimitiveComponent.SetCollisionEnabled` wheel "QueryAndPhysics")
  (`PrimitiveComponent.SetSimulatePhysics` wheel true))

(fn `FrontTracer`
  (locals (NewLocalVar_0 :type Boolean :default false))
  (bind _tracefront (`self.TraceFront`))
  (bind _trace_fr (`self.Trace_FR`))
  (bind _trace_fl (`self.Trace_FL`))
  (bind _returnvalue (`SceneComponent.K2_GetComponentLocation` _tracefront))
  (bind _returnvalue_2 (`SceneComponent.K2_GetComponentLocation` _trace_fl))
  (bind _returnvalue_3 (`SceneComponent.K2_GetComponentLocation` _trace_fr))
  (bind (_outhits _returnvalue_4) (`KismetSystemLibrary.LineTraceMulti` _returnvalue (+ _returnvalue (* (`SceneComponent.GetForwardVector` _tracefront) 600.0)) "TraceTypeQuery1"))
  (bind (_outhits_2 _returnvalue_5) (`KismetSystemLibrary.LineTraceMulti` _returnvalue_3 (+ _returnvalue_3 (* (`SceneComponent.GetForwardVector` _trace_fr) 400.0)) "TraceTypeQuery1"))
  (bind (_outhits_3 _returnvalue_6) (`KismetSystemLibrary.LineTraceMulti` _returnvalue_2 (+ _returnvalue_2 (* (`SceneComponent.GetForwardVector` _trace_fl) 400.0)) "TraceTypeQuery1"))
  (if _returnvalue_6
    (set `self.AI_Steering` -1.0)
    (else
      (set `self.AI_Steering` 1.0)))
  (set `self.FrontTraceHit` (or (or _returnvalue_4 _returnvalue_5) _returnvalue_6)))

(fn `GetSpeedKMH`
  (returns (speed :type "Float (double-precision)"))
  (return (* (`ChaosVehicleMovementComponent.GetForwardSpeed` (`self.VehicleMovementComponent`)) 0.036)))

(fn `OnRep_DisplayName`
  (`TextRenderComponent.K2_SetText` (`self.TextRender`) (`KismetTextLibrary.Conv_StringToText` (`self.DisplayName`))))

(fn `SetAI`
  (params (throttle :type "Float (double-precision)") (brake :type "Float (double-precision)") (steer :type "Float (double-precision)"))
  (bind _vehiclemovementcomponent (`self.VehicleMovementComponent`))
  (`ChaosVehicleMovementComponent.SetThrottleInput` _vehiclemovementcomponent throttle)
  (`ChaosVehicleMovementComponent.SetBrakeInput` _vehiclemovementcomponent brake)
  (`ChaosVehicleMovementComponent.SetSteeringInput` _vehiclemovementcomponent steer)
  (`self.BrakeLights` (> brake 0.0)))

(fn `SetLights`
  (params (lights :type "Float (double-precision)"))
  (bind _output_get (set `self.FrontLight` lights))
  (`self.UpdateMaterial_Server` (`self.BrakeLight`) (`self.ColorBody`) _output_get))

(fn `SetPaint`
  (params (color :type "LinearColor Structure"))
  (bind _output_get (set `self.ColorBody` color))
  (`self.UpdateMaterial_Server` (`self.BrakeLight`) _output_get (`self.FrontLight`)))

(fn `ShowName`
  (params (Show :type Boolean))
  (`SceneComponent.SetVisibility` (`self.TextRender`) Show false))

(fn `UserConstructionScript`)