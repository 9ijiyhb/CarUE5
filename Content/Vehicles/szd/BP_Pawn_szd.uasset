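; Networked player vehicle pawn (szd) with throttle, steering, handbrake, an orbiting spring-arm camera and a front/back camera switch.
; Brake light, headlight and body color changes pass through a server event to a multicast that updates a dynamic material instance.
; Reset has the server ask VehicleAdvGameMode to respawn the car just above its position, keeping yaw.
; A RepNotify DisplayName feeds a name text, hidden at BeginPlay; several disconnected respawn experiments remain.
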(event `UpdateMaterial_Server`
  (params (brake :type "Float (double-precision)") (body_c :type "LinearColor Structure") (Light :type "Float (double-precision)"))
  (`self.UpdateMaterial_Multicast` brake body_c Light))

(event `UpdateMaterial_Multicast`
  (params (Brake :type "Float (double-precision)") (body_c :type "LinearColor Structure") (Light :type "Float (double-precision)"))
  (bind _matbody (`self.MatBody`)
    (:`then`
      (`MaterialInstanceDynamic.SetScalarParameterValue` _matbody "BrakeLightPower" Brake)
      (`MaterialInstanceDynamic.SetVectorParameterValue` _matbody "BodyColor" body_c)
      (`MaterialInstanceDynamic.SetScalarParameterValue` _matbody "FrontLightPower" Light))
    (:`else`)))

(event `UpdateMaterial`
  (`/Engine/EditorBlueprintResources/ActorMacros.Switch Has Authority`
    (:`Authority`
      (`self.UpdateMaterial_Multicast` 0.0))
    (:`Remote`
      (`self.UpdateMaterial_Server` 0.0))))

(event `self.ReceiveBeginPlay`
  ;[1 1 1] Comment
  (bind _returnvalue (`PrimitiveComponent.CreateDynamicMaterialInstance` (`self.Mesh`) 0 "/Game/Vehicles/szd/mat_szd_base_Inst.mat_szd_base_Inst" "None"))
  (set `self.MatBody` _returnvalue)
  (`self.UpdateMaterial_Server` (`self.BrakeLight`) (`self.ColorBody`) (`self.FrontLight`))
  (`self.respawn_init` (`AdvancedIdentityLibrary.GetPlayerNickname` (`AdvancedSessionsLibrary.GetUniqueNetID` (`GameplayStatics.GetPlayerController` 0))))
  (`self.ShowName` false))

(event `InputAxis|MoveForward`
  (params (AxisValue :type "Float (single-precision)"))
  (bind _vehiclemovementcomponent (`self.VehicleMovementComponent`))
  (bind _vehiclemovementcomponent_2 (`self.VehicleMovementComponent`))
  ;[1 1 1] Movement control
  (if (>= AxisValue 0.0)
    (`ChaosVehicleMovementComponent.SetThrottleInput` _vehiclemovementcomponent AxisValue)
    (`ChaosVehicleMovementComponent.SetBrakeInput` _vehiclemovementcomponent 0.0)
    (`/Engine/EditorBlueprintResources/StandardMacros.DoOnce` false :!label _label
      (:`Completed`
        (`self.BrakeLights` false)))
    (else
      (`ChaosVehicleMovementComponent.SetBrakeInput` _vehiclemovementcomponent_2 (* AxisValue -1.0))
      (`ChaosVehicleMovementComponent.SetThrottleInput` _vehiclemovementcomponent_2 0.0)
      (`self.BrakeLights` true)
      (goto _label :!via `Reset`))))

(event `respawn_init`
  (params (name :type String))
  (set `self.DisplayName` name))

(event `InputAxis|MoveRight`
  (params (AxisValue :type "Float (single-precision)"))
  ;[1 1 1] Movement control
  (`ChaosVehicleMovementComponent.SetSteeringInput` (`self.VehicleMovementComponent`) AxisValue))

(event `InputAction|Handbrake`
  (params (Key :type "Key Structure"))
  (bind _vehiclemovementcomponent (`self.VehicleMovementComponent`))
  ;[1 1 1] Movement control
  (:`Pressed`
    (`ChaosVehicleMovementComponent.SetHandbrakeInput` _vehiclemovementcomponent true)
    (`self.BrakeLights` true))
  (:`Released`
    (`ChaosVehicleMovementComponent.SetHandbrakeInput` _vehiclemovementcomponent false)
    (`self.BrakeLights` false)))

(event `InputAction|SwitchLight`
  (params (Key :type "Key Structure"))
  (:`Pressed`
    (bind _output_get (set `self.FrontLight` 15.0))
    (`self.UpdateMaterial_Server` (`self.BrakeLight`) (`self.ColorBody`) _output_get)
    (`/Engine/EditorBlueprintResources/ActorMacros.Switch Has Authority`
      (:`Authority`
        (set `self.DisplayName` "XAXA")))))

(event `InputAxis|LookRight`
  (params (AxisValue :type "Float (single-precision)"))
  (bind _springarm (`self.SpringArm`))
  (bind (_relativerotation_roll _relativerotation_pitch _relativerotation_yaw) (`KismetMathLibrary.BreakRotator` (`SceneComponent.RelativeRotation` (`self.SpringArm`))))
  ;[1 1 1] Camera Control
  (if (!= AxisValue 0.0)
    (`SceneComponent.K2_AddLocalRotation` _springarm (`KismetMathLibrary.MakeRotator` 0.0 0.0 AxisValue) false false) ; Rotate camera around the vehicle
    (else
      (`SceneComponent.K2_SetRelativeRotation` _springarm (`KismetMathLibrary.MakeRotator` 0.0 0.0 (`KismetMathLibrary.FInterpTo` _relativerotation_yaw 0.0 (`GameplayStatics.GetWorldDeltaSeconds`) 1.0)) false false) ; Reset camera to original angle
    )))

(event `InputAction|color_test`
  (params (Key :type "Key Structure"))
  (:`Pressed`
    (bind _output_get (set `self.ColorBody` (make `LinearColor` (`KismetMathLibrary.RandomFloatInRange` 0.0 1.0) (`KismetMathLibrary.RandomFloatInRange` 0.0 1.0) (`KismetMathLibrary.RandomFloatInRange` 0.0 1.0) 1.0)))
    (`self.UpdateMaterial_Server` (`self.BrakeLight`) _output_get)
    (set `self.FrontLight` 0.0)))

(event `InputAction|SwitchCamera`
  (params (Key :type "Key Structure"))
  ;[1 1 1] Camera Control
  (:`Pressed`
    (`ActorComponent.Deactivate` (`self.BackCamera`))
    (`ActorComponent.Deactivate` (`self.FrontCamera`))
    (`/Engine/EditorBlueprintResources/StandardMacros.FlipFlop`
      (:`A`
        (`ActorComponent.Activate` (`self.FrontCamera`) false))
      (:`B`
        (`ActorComponent.Activate` (`self.BackCamera`) false)))))

(event `InputAction|ResetCar`
  (params (Key :type "Key Structure"))
  (:`Pressed`
    (`/Engine/EditorBlueprintResources/ActorMacros.Switch Has Authority`
      (:`Authority`
        _)
      (:`Remote`
        _))
    (`self.reset` (`GameplayStatics.GetPlayerController` 0))))

(event `reset`
  (params (controll :type "PlayerController Object Reference"))
  (bind (_returnvalue_roll _returnvalue_pitch _returnvalue_yaw) (`KismetMathLibrary.BreakRotator` (`self.K2_GetActorRotation`)))
  (bind _returnvalue (`GameplayStatics.GetGameMode`))
  ;[1 1 1] Comment
  (`/Engine/EditorBlueprintResources/ActorMacros.Switch Has Authority`
    (:`Authority`
      (`/Engine/EditorBlueprintResources/StandardMacros.IsValid` _returnvalue
        (:`Is Valid`
          (bind _asvehicle_adv_game_mode (cast `/Game/VehicleTemplate/Blueprints/VehicleAdvGameMode` _returnvalue))
          (`/Game/VehicleTemplate/Blueprints/VehicleAdvGameMode.respawn` _asvehicle_adv_game_mode controll (`KismetMathLibrary.MakeTransform` (+ (`self.K2_GetActorLocation`) (0.0 0.0 250.0)) (`KismetMathLibrary.MakeRotator` 0.0 0.0 _returnvalue_yaw)))
          (`KismetSystemLibrary.PrintString` "reset !"))))))

(fn `BrakeLights`
  (params (BrakeLights :type Boolean))
  (bind _frontlight (`self.FrontLight`))
  (bind _colorbody (`self.ColorBody`))
  (if BrakeLights
    (bind _output_get (set `self.BrakeLight` 6.0))
    (`self.UpdateMaterial_Server` _output_get _colorbody _frontlight)
    (else
      (bind _output_get_2 (set `self.BrakeLight` 0.0))
      (`self.UpdateMaterial_Server` _output_get_2 _colorbody _frontlight))))

(fn `OnRep_DisplayName`
  (`TextRenderComponent.K2_SetText` (`self.TextRender`) (`KismetTextLibrary.Conv_StringToText` (`self.DisplayName`))))

(fn `SetLights`
  (params (lights :type "Float (double-precision)"))
  (bind _output_get (set `self.FrontLight` lights))
  (`self.UpdateMaterial_Server` (`self.BrakeLight`) (`self.ColorBody`) _output_get))

(fn `SetPaint`
  (params (color :type "LinearColor Structure"))
  (bind _output_get (set `self.ColorBody` color))
  (`self.UpdateMaterial_Server` (`self.BrakeLight`) _output_get (`self.FrontLight`)))

(fn `ShowName`
  (params (Show :type Boolean))
  (`SceneComponent.SetVisibility` (`self.TextRender`) Show false))

(fn `UserConstructionScript`)