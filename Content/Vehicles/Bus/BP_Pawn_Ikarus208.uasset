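; Drivable Ikarus 208 bus vehicle pawn that takes player throttle, steering, handbrake and spring-arm camera input, or drives itself when IsAI is set.
; In AI mode, each tick steers toward a look-ahead point on the Path spline under a speed limiter that brakes at the limit.
; Two forward line traces override lane following on a hit, setting fixed steering with reduced throttle, or braking if moving backward.
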(event `self.ReceiveBeginPlay`
  (set `self.AI_Throttle` 1.0))

(event `InputAxis|MoveForward`
  (params (AxisValue :type "Float (single-precision)"))
  (bind _vehiclemovementcomponent (`self.VehicleMovementComponent`))
  (bind _vehiclemovementcomponent_2 (`self.VehicleMovementComponent`))
  ;[0.5117 0.7258 1] CONTROL
  (if (`self.isAI`)
    _
    (elif (>= AxisValue 0.0)
      (`ChaosVehicleMovementComponent.SetThrottleInput` _vehiclemovementcomponent AxisValue)
      (`ChaosVehicleMovementComponent.SetBrakeInput` _vehiclemovementcomponent 0.0)
      (else
        (`ChaosVehicleMovementComponent.SetBrakeInput` _vehiclemovementcomponent_2 (* AxisValue -1.0))
        (`ChaosVehicleMovementComponent.SetThrottleInput` _vehiclemovementcomponent_2 0.0)))))

(event `InputAxis|MoveRight`
  (params (AxisValue :type "Float (single-precision)"))
  ;[0.5117 0.7258 1] CONTROL
  (if (not (`self.isAI`))
    (`ChaosVehicleMovementComponent.SetSteeringInput` (`self.VehicleMovementComponent`) AxisValue)))

(event `InputAction|Handbrake`
  (params (Key :type "Key Structure"))
  (bind _vehiclemovementcomponent (`self.VehicleMovementComponent`))
  ;[0.5117 0.7258 1] CONTROL
  (:`Pressed`
    (`ChaosVehicleMovementComponent.SetHandbrakeInput` _vehiclemovementcomponent true))
  (:`Released`
    (`ChaosVehicleMovementComponent.SetHandbrakeInput` _vehiclemovementcomponent false)))

(event `self.ReceiveTick`
  (params (DeltaSeconds :type "Float (single-precision)"))
  ;[1 1 1] Comment
  (if (`self.isAI`)
    (`self.FrontTracer`)
    (if (`self.Front Trace Hit`)
      (if (< (`self.GetSpeedKMH`) 0.0)
        (`self.SetAI` 0.0 15.0 15.0)
        (else
          (`self.SetAI` (* (`self.AI_Throttle`) 0.25) 0.0 -5.0)))
      (else
        (`self.Speed Limiter` (`self.Speed Limit KMH`)
          (:`then`
            (bind _steering (`self.AILane` (`self.path`)))
            (`self.SetAI` (`self.AI_Throttle`) 0.0 _steering))
          (:`false`
            (`self.SetAI` 0.0 15.0)))))
    (else
      (`self.NewFunction_0`))))

(event `InputAxis|LookUp`
  (params (AxisValue :type "Float (single-precision)"))
  (bind (_returnvalue_roll _returnvalue_pitch _returnvalue_yaw) (`KismetMathLibrary.BreakRotator` (`SceneComponent.K2_GetComponentRotation` (`self.SpringArm`))))
  ;[0.3438 1 1] Camera
  (if (> (`KismetMathLibrary.Abs` _returnvalue_pitch) 50.0) :!label _label
    (`SceneComponent.K2_SetWorldRotation` (`self.SpringArm`) (`KismetMathLibrary.RInterpTo` (`KismetMathLibrary.MakeRotator` _returnvalue_roll _returnvalue_pitch _returnvalue_yaw) (`KismetMathLibrary.MakeRotator` _returnvalue_roll 0.0 _returnvalue_yaw) (`GameplayStatics.GetWorldDeltaSeconds`) 1.0) false false)
    (else
      (`SceneComponent.K2_AddRelativeRotation` (`self.SpringArm`) (`KismetMathLibrary.MakeRotator` 0.0 AxisValue (stale `InputAxis|LookRight` AxisValue)) false false))))

(event `InputAxis|LookRight`
  (params (AxisValue :type "Float (single-precision)"))
  ;[0.3438 1 1] Camera
  (goto _label))

(fn `AILane`
  (params (path :type "/Game/AI/LanePath Object Reference"))
  (returns (steering :type "Float (double-precision)"))
  (bind _returnvalue (`self.K2_GetActorLocation`))
  (bind _spline (`/Game/AI/LanePath.Spline` path))
  (bind (_returnvalue_roll _returnvalue_pitch _returnvalue_yaw) (`KismetMathLibrary.BreakRotator` (`KismetMathLibrary.NormalizedDeltaRotator` (`KismetMathLibrary.FindLookAtRotation` _returnvalue (`SplineComponent.FindLocationClosestToWorldLocation` _spline (+ (* (`KismetMathLibrary.Normal` (`SplineComponent.FindTangentClosestToWorldLocation` _spline _returnvalue "World")) 500.0) _returnvalue) "World")) (`self.K2_GetActorRotation`))))
  (return (`KismetMathLibrary.MapRangeClamped` _returnvalue_yaw -90.0 90.0 -5.0 5.0)))

(fn `FrontTracer`
  (bind _trace1 (`self.Trace1`))
  (bind _trace2 (`self.Trace2`))
  (bind _returnvalue (`SceneComponent.K2_GetComponentLocation` _trace1))
  (bind _returnvalue_2 (`SceneComponent.K2_GetComponentLocation` _trace2))
  (bind (_outhits _returnvalue_3) (`KismetSystemLibrary.LineTraceMulti` :`Start` _returnvalue :`End` (+ _returnvalue (* (`SceneComponent.GetForwardVector` _trace1) 600.0)) :`TraceChannel` "TraceTypeQuery1" :`DrawDebugType` "ForOneFrame"))
  (bind (_outhits_2 _returnvalue_4) (`KismetSystemLibrary.LineTraceMulti` :`Start` _returnvalue_2 :`End` (+ _returnvalue_2 (* (`SceneComponent.GetForwardVector` _trace2) 400.0)) :`TraceChannel` "TraceTypeQuery1" :`DrawDebugType` "ForOneFrame"))
  (bind _output_get (set `self.Front Trace Hit` (or _returnvalue_3 _returnvalue_4)))
  (if _output_get
    (set `self.AI_Sterring` 15.0)))

(fn `GetSpeedKMH`
  (returns (speed :type "Float (double-precision)"))
  (return (* (`ChaosVehicleMovementComponent.GetForwardSpeed` (`self.VehicleMovementComponent`)) 0.036)))

(fn `NewFunction_0`
  (`SceneComponent.K2_AddRelativeRotation` (`self.SpringArm`) (`KismetMathLibrary.MakeRotator` 0.0 (`self.GetInputAxisValue`) (`self.GetInputAxisValue`)) false false))

(fn `SetAI`
  (params (throttle :type "Float (double-precision)") (brake :type "Float (double-precision)") (steer :type "Float (double-precision)"))
  (bind _vehiclemovementcomponent (`self.VehicleMovementComponent`))
  (`ChaosVehicleMovementComponent.SetThrottleInput` _vehiclemovementcomponent throttle)
  (`ChaosVehicleMovementComponent.SetBrakeInput` _vehiclemovementcomponent brake)
  (`ChaosVehicleMovementComponent.SetSteeringInput` _vehiclemovementcomponent steer))

(fn `UserConstructionScript`)